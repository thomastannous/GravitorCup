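; BP_GBall is the game ball's presentation layer, turning possession, spin, lift, expiration and collisions into visuals, audio and camera shake.
; Tick drives emissive colors on dynamic ball and ring materials, spin-scaled shake and sound, and a sine wobble of the mesh at high speed.
; Gravitor hits recolor the ball and spawn oriented Niagara bursts when hard, while other hits play collision audio.
; Ball events trigger possession VFX and audio fades.
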(event `self.ReceiveBeginPlay`
  (bind _returnvalue (`PrimitiveComponent.CreateDynamicMaterialInstance` (`self.BallMesh`) 0 null "None"))
  (set `self.BallMatInst` _returnvalue)
  (bind _returnvalue_2 (`PrimitiveComponent.CreateDynamicMaterialInstance` (`self.InnerRing`) 0 "/Game/LevelContent/Ball/Visuals/M_Ring.M_Ring" "None"))
  (set `self.InnerRingMatInst` _returnvalue_2)
  (bind _returnvalue_3 (`PrimitiveComponent.CreateDynamicMaterialInstance` (`self.OuterRing`) 0 "/Game/LevelContent/Ball/Visuals/M_Ring.M_Ring" "None"))
  (set `self.OuterRingMatInst` _returnvalue_3)
  (`AudioComponent.Stop` (`self.SpinRelease`)))

(event `self.ReceiveTick`
  (params (DeltaSeconds :type "Float (single-precision)"))
  (`KismetSystemLibrary.PrintString` (`KismetStringLibrary.Conv_DoubleToString` (`self.Expiration`)) true true (struct :`G` 0.66 :`B` 1.0 :`A` 1.0) DeltaSeconds)
  (`self.TickSFX` DeltaSeconds)
  (`self.TickVFX` DeltaSeconds)
  (if (and (`KismetSystemLibrary.IsValid` (`self.BallMatInst`)) (`KismetSystemLibrary.IsValid` (`self.InnerRingMatInst`)) (`KismetSystemLibrary.IsValid` (`self.OuterRingMatInst`)))
    (`self.SpinTick` DeltaSeconds)
    (`self.LiftTick` DeltaSeconds)
    (bind _returnvalue (`PrimitiveComponent.GetPhysicsLinearVelocity` (`self.CollisionSphere`) "None"))
    (bind _returnvalue_2 (`KismetMathLibrary.VSize` _returnvalue))
    (if (and (== (`KismetArrayLibrary.Array_Length` (`self.PendingGravityForces`)) 0) (> _returnvalue_2 3000.0))
      (`SceneComponent.K2_SetRelativeLocation` (`self.BallMesh`) (* (`KismetMathLibrary.Normal` (`KismetMathLibrary.RotateAngleAxis` _returnvalue 90.0 (0.0 0.0 1.0))) (* (`KismetMathLibrary.NormalizeToRange` _returnvalue_2 3000.0 5000.0) (* (`KismetMathLibrary.Sin` (* (`GameplayStatics.GetTimeSeconds`) 20.0)) 17.0))) false false)
      (else
        (`SceneComponent.K2_SetRelativeLocation` (`self.BallMesh`) (0.0 0.0 0.0) false false)))))

(event `TickVFX`
  (params (DeltaTime :type "Float (double-precision)")))

(event `self.OnBallChangePossession`
  (params (Team :type Integer))
  (bind _possessionchangevfx (`self.PossessionChangeVFX`))
  (if (!= Team -1)
    (`NiagaraComponent.SetVariableLinearColor` _possessionchangevfx "PossessingTeam" (`KismetMathLibrary.SelectColor` (make `LinearColor` 25.0 10.0 1.0 1.0) (make `LinearColor` 1.0 1.0 25.0 1.0) (`KismetMathLibrary.Conv_IntToBool` Team)))
    (`NiagaraComponent.ResetSystem` _possessionchangevfx)
    (`ActorComponent.Activate` _possessionchangevfx false)))

(event `self.OnResetBall`
  (`AudioComponent.FadeIn` (`self.Movement`) 0.0 1.0 0.0 "Linear")
  (`AudioComponent.FadeIn` (`self.SpinRelease`) 0.0 1.0 0.0 "Linear")
  (`AudioComponent.FadeIn` (`self.CollisionSFX`) 0.0 1.0 0.0 "Linear")
  (`AudioComponent.FadeIn` (`self.SpinLoad`) 0.0 1.0 0.0 "Linear"))

(event `SpinTick`
  (params (DeltaTime :type "Float (double-precision)"))
  (bind _returnvalue (`KismetMathLibrary.NormalizeToRange` (`self.SpinVelLength`) 0.0 100.0))
  (bind _playercameramanager (`PlayerController.PlayerCameraManager` (`GameplayStatics.GetPlayerController` 0)))
  (bind _output_get (set `self.SpinVelLength` (`KismetMathLibrary.VSize` (`self.SpinVelocity`))))
  (bind _returnvalue_2 (`KismetMathLibrary.MapRangeClamped` _output_get 0.0 (`self.MaxSpinSpeed`) 0.0 5000.0))
  (`MaterialInstanceDynamic.SetVectorParameterValue` (`self.InnerRingMatInst`) "EmissiveColor" (`KismetMathLibrary.MakeColor` _returnvalue_2 _returnvalue_2 _returnvalue_2))
  (bind _returnvalue_3 (`MaterialInstanceDynamic.K2_GetVectorParameterValue` (`self.BallMatInst`) "EmissiveColor"))
  (`MaterialInstanceDynamic.SetVectorParameterValue` (`self.BallMatInst`) "EmissiveColor" (`KismetMathLibrary.LinearColorLerp` _returnvalue_3 (* (`KismetMathLibrary.SelectColor` (struct :`R` 0.039516 :`G` 0.0376 :`B` 1.0 :`A` 1.0) (struct :`R` 1.0 :`G` 0.821741 :`A` 1.0) (< (`self.Expiration`) 0.0)) (`CurveLinearColor.GetLinearColorValue` (`self.ExpirationGlow`) (- 1.0 (`KismetMathLibrary.NormalizeToRange` (`KismetMathLibrary.Abs` (`self.Expiration`)) 0.0 (`self.ExpirationTime`))))) DeltaTime))
  (if (> _returnvalue 0.0)
    (`|ExecutionSequence`
      (:`then_0`
        (`/Engine/EditorBlueprintResources/StandardMacros.DoOnce` false :!label _label
          (:`Completed`
            (bind _returnvalue_4 (`PlayerCameraManager.StartMatineeCameraShake` :`self` _playercameramanager :`ShakeClass` "/Game/LevelContent/Ball/CamShake_BallSpin.CamShake_BallSpin_C" :`Scale` _returnvalue)))))
      (:`then_1`
        (set `MatineeCameraShake.ShakeScale` _returnvalue _returnvalue_4)))
    (else
      (`|ExecutionSequence`
        (:`then_0`
          (goto _label :!via `Reset`))
        (:`then_1`
          (`PlayerCameraManager.StopCameraShake` _playercameramanager _returnvalue_4 true))))))

(event `LiftTick`
  (params (DeltaTime :type "Float (double-precision)"))
  (bind _returnvalue (`KismetMathLibrary.SelectColor` (struct :`R` 0.592713 :`G` 0.564002 :`B` 15.0 :`A` 1.0) (struct :`R` 15.0 :`G` 12.326119 :`A` 1.0) (== (`self.PossessingTeam`) 0)))
  (bind _returnvalue_2 (`KismetMathLibrary.SelectColor` (struct :`R` 1.0 :`G` 1.0 :`B` 1.0 :`A` 1.0) _returnvalue (== (`self.PossessingTeam`) -1)))
  (`MaterialInstanceDynamic.SetVectorParameterValue` (`self.OuterRingMatInst`) "EmissiveColor" (`KismetMathLibrary.SelectColor` (struct :`R` 1.0 :`G` 1.0 :`B` 1.0 :`A` 1.0) _returnvalue (`self.Lifted`)))
  (bind _returnvalue_3 (`MaterialInstanceDynamic.K2_GetVectorParameterValue` (`self.BallMatInst`) "EmissiveColor"))
  (`MaterialInstanceDynamic.SetVectorParameterValue` (`self.BallMatInst`) "EmissiveColor" (`KismetMathLibrary.LinearColorLerp` _returnvalue_3 (* (`KismetMathLibrary.SelectColor` (+ (`self.LiftRingColor`) _returnvalue_2) _returnvalue_2 (`self.Lifted`)) (`KismetMathLibrary.SelectFloat` 6000.0 1.0 (`self.bIsDeadly`))) (* 12.0 DeltaTime))))

(event `self.CollisionSphere.OnComponentHit`
  (params (HitComponent :type "PrimitiveComponent Object Reference") (OtherActor :type "Actor Object Reference") (OtherComp :type "PrimitiveComponent Object Reference") (NormalImpulse :type "Vector Structure") (Hit :type "HitResult Structure (by ref)"))
  (bind (_bblockinghit _binitialoverlap _time _distance _location _impactpoint _normal) (`GameplayStatics.BreakHitResult` Hit))
  (bind _returnvalue (`SceneComponent.K2_GetComponentLocation` (`self.CollisionSphere`)))
  (bind _asbp_gravitor (cast `/Game/Player/BaseGravitor/BP_Gravitor` OtherActor)
    (:`then`
      (`MaterialInstanceDynamic.SetVectorParameterValue` (`self.BallMatInst`) "BallColor" (`GGravitor.GravitorColor` _asbp_gravitor))
      (if (> (`KismetMathLibrary.VSize` NormalImpulse) 2500.0)
        (bind _returnvalue_2 (`PrimitiveComponent.GetPhysicsLinearVelocity` (`self.CollisionSphere`) "None"))
        (bind _returnvalue_3 (`PrimitiveComponent.GetPhysicsLinearVelocity` OtherComp "None"))
        (bind _returnvalue_4 (`NiagaraFunctionLibrary.SpawnSystemAtLocation` "/Game/Player/BaseGravitor/VFX/Collision/NS_Collision.NS_Collision" _location (`KismetMathLibrary.MakeRotFromX` (`KismetMathLibrary.RotateAngleAxis` _normal (`KismetMathLibrary.SelectFloat` -90.0 90.0 (> (`KismetMathLibrary.Dot_VectorVector` (- _returnvalue_3 _returnvalue_2) (`KismetMathLibrary.RotateAngleAxis` (- _location _returnvalue) 90.0 (0.0 0.0 1.0))) 0.0)) (0.0 0.0 1.0))) (1.0 1.0 1.0) true false))
        (`NiagaraComponent.SetVariableVec3` _returnvalue_4 "GravitorLoc" _returnvalue)
        (`ActorComponent.Activate` _returnvalue_4 false)))
    (:`CastFailed`
      (`ActorComponent.Activate` (`self.CollisionSFX`) false)
      (`AudioComponent.Play` (`self.CollisionSFX`) 0.0))))

(event `TickSFX`
  (params (DeltaTime :type "Float (double-precision)"))
  (bind _returnvalue (`KismetMathLibrary.VSize` (`self.SpinVelocity`)))
  (bind _returnvalue_2 (`KismetMathLibrary.VSize` (`self.SpinVelocity`)))
  (`self.TickSFXMOvement`)
  (`AudioComponent.SetPitchMultiplier` (`self.SpinLoad`) (`KismetMathLibrary.MapRangeClamped` _returnvalue_2 0.0 100.0 0.8 1.0))
  (`AudioComponent.SetVolumeMultiplier` (`self.SpinLoad`) (`KismetMathLibrary.MapRangeClamped` _returnvalue_2 0.0 50.0 0.0 1.0))
  (if (not (`self.Lifted`))
    (`|ExecutionSequence`
      (:`then_0`
        (if (`KismetMathLibrary.NearlyEqual_FloatFloat` _returnvalue)
          (`AudioComponent.FadeOut` (`self.SpinRelease`) 0.0 0.0 "Linear")))
      (:`then_1`
        (`AudioComponent.SetVolumeMultiplier` (`self.SpinRelease`) (`KismetMathLibrary.MapRangeClamped` _returnvalue 0.0 5.0 0.0 1.0))
        (`AudioComponent.SetPitchMultiplier` (`self.SpinRelease`) (`KismetMathLibrary.MapRangeClamped` _returnvalue 0.0 100.0 0.5 1.5))))))

(event `self.OnGrounded`
  (`AudioComponent.FadeIn` (`self.SpinRelease`) 0.1 1.0 0.0 "Linear"))

(event `self.OnLifted`
  (`AudioComponent.FadeOut` (`self.SpinRelease`) 0.0 0.0 "Linear"))

(event `TickSFXMovement`
  (bind _returnvalue (`PrimitiveComponent.GetPhysicsLinearVelocity` (`self.CollisionSphere`) "None"))
  (bind _returnvalue_2 (`KismetMathLibrary.VSize` _returnvalue))
  (`AudioComponent.SetVolumeMultiplier` (`self.Movement`) (`KismetMathLibrary.MapRangeClamped` _returnvalue_2 0.0 4000.0 0.0 0.3))
  (`AudioComponent.SetPitchMultiplier` (`self.Movement`) (`KismetMathLibrary.MapRangeClamped` _returnvalue_2 0.0 4000.0 0.8 1.2)))

(event `self.OnBallExpired`
  (`AudioComponent.FadeOut` (`self.SpinLoad`) 0.1 0.0 "Linear")
  (`AudioComponent.FadeOut` (`self.Movement`) 0.1 0.0 "Linear")
  (`AudioComponent.FadeOut` (`self.CollisionSFX`) 0.1 0.0 "Linear")
  (`AudioComponent.FadeOut` (`self.SpinRelease`) 0.1 0.0 "Linear"))

(fn `UserConstructionScript`)