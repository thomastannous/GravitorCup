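; BP_Gravitor is the player's Gravitor, handling its look, sound and collision feedback around gravity and ball-attraction state.
; Tick spins the capsule by gravity state, trails the ball mesh behind the ring, and drives gravity audio fades and parameters.
; Capsule hits scale audio by impulse, with strong hits adding Niagara sparks, camera shake and force feedback.
; A SoundPlayed handshake prevents doubled sounds between colliding Gravitors, and BeginPlay hue-shifts the ring by team.
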(event `self.ReceiveBeginPlay`
  (`KismetSystemLibrary.Delay` 0.2)
  (bind _returnvalue (`PrimitiveComponent.CreateDynamicMaterialInstance` (`self.RingMesh`) 0 "/Game/Player/BaseGravitor/Visuals/M_BaseGravitor.M_BaseGravitor" "None"))
  (set `self.BallMatInst` _returnvalue)
  (bind _asbp_gplayer_controller (cast `/Game/Framework/PlayerController/BP_GPlayerController` (`self.GetController`)))
  (if (== (`GPlayerController.Team` _asbp_gplayer_controller) 0)
    (`MaterialInstanceDynamic.SetScalarParameterValue` (`self.BallMatInst`) "HueShift" 0.60438))
  (`AudioComponent.Stop` (`self.sg_GravityActive`))
  (`AudioComponent.Stop` (`self.CollisionAudio`)))

(event `self.ReceiveTick`
  (params (DeltaSeconds :type "Float (single-precision)"))
  (`self.TickSFX`)
  (`self.TickVFX` DeltaSeconds)
  (`SceneComponent.K2_AddRelativeRotation` (`self.CollisionCapsule`) (* (`KismetMathLibrary.SelectRotator` (`KismetMathLibrary.MakeRotator` 0.0 0.0 -60.0) (`KismetMathLibrary.MakeRotator` 0.0 0.0 -120.0) (`self.bIsGravityActive`)) DeltaSeconds) false false)
  (`SceneComponent.K2_SetWorldLocation` (`self.BallMesh`) (`KismetMathLibrary.MakeVector` (.x (`KismetMathLibrary.VInterpTo` (`SceneComponent.K2_GetComponentLocation` (`self.BallMesh`)) (`SceneComponent.K2_GetComponentLocation` (`self.RingMesh`)) DeltaSeconds (`self.BallLerpSpeed`))) (.y (`KismetMathLibrary.VInterpTo` (`SceneComponent.K2_GetComponentLocation` (`self.BallMesh`)) (`SceneComponent.K2_GetComponentLocation` (`self.RingMesh`)) DeltaSeconds (`self.BallLerpSpeed`))) (.z (`SceneComponent.K2_GetComponentLocation` (`self.BallMesh`)))) false false))

(event `self.CollisionCapsule.OnComponentHit`
  (params (HitComponent :type "PrimitiveComponent Object Reference") (OtherActor :type "Actor Object Reference") (OtherComp :type "PrimitiveComponent Object Reference") (NormalImpulse :type "Vector Structure") (Hit :type "HitResult Structure (by ref)"))
  (bind _returnvalue (`KismetMathLibrary.VSize` NormalImpulse))
  (bind (_bblockinghit _binitialoverlap _time _distance _location _impactpoint _normal) (`GameplayStatics.BreakHitResult` Hit))
  (bind _collisionaudio (`self.CollisionAudio`))
  (bind _returnvalue_2 (> _returnvalue 2500.0))
  (bind _returnvalue_3 (`SceneComponent.K2_GetComponentLocation` (`self.CollisionCapsule`)))
  (bind _asbp_gravitor (cast `/Game/Player/BaseGravitor/BP_Gravitor` OtherActor)
    (:`then`
      (if (not (`/Game/Player/BaseGravitor/BP_Gravitor.SoundPlayed` _asbp_gravitor))
        (set `self.SoundPlayed` true)
        (`AudioComponent.SetVolumeMultiplier` (`self.CollisionAudio`) (`KismetMathLibrary.NormalizeToRange` _returnvalue 0.0 5000.0) :!label _label)
        (if _returnvalue_2
          (`AudioComponent.SetBoolParameter` _collisionaudio "WeakCollision" false)
          (`AudioComponent.Play` _collisionaudio 0.0)
          (`|ExecutionSequence`
            (:`then_0`
              (bind _returnvalue_4 (`PrimitiveComponent.GetPhysicsLinearVelocity` (`self.CollisionCapsule`) "None" :!label _label_2))
              (bind _returnvalue_5 (`PrimitiveComponent.GetPhysicsLinearVelocity` OtherComp "None"))
              (bind _returnvalue_6 (`NiagaraFunctionLibrary.SpawnSystemAtLocation` "/Game/Player/BaseGravitor/VFX/Collision/NS_Collision.NS_Collision" _location (`KismetMathLibrary.MakeRotFromX` (`KismetMathLibrary.RotateAngleAxis` _normal (`KismetMathLibrary.SelectFloat` -90.0 90.0 (> (`KismetMathLibrary.Dot_VectorVector` (- _returnvalue_5 _returnvalue_4) (`KismetMathLibrary.RotateAngleAxis` (- _location _returnvalue_3) 90.0 (0.0 0.0 1.0))) 0.0)) (0.0 0.0 1.0))) (1.0 1.0 1.0) true false))
              (`NiagaraComponent.SetVariableVec3` _returnvalue_6 "GravitorLoc" _returnvalue_3)
              (`ActorComponent.Activate` _returnvalue_6 false)
              (`PlayerCameraManager.PlayCameraShake` :`self` (`PlayerController.PlayerCameraManager` (`GameplayStatics.GetPlayerController` 0)) :`ShakeClass` "/Game/Framework/ArenaCamera/CS_Collision.CS_Collision_C" :`Scale` (`KismetMathLibrary.NormalizeToRange` (`KismetMathLibrary.VSize` NormalImpulse) 0.0 7000.0))
              (bind _asbp_gplayer_controller (cast `/Game/Framework/PlayerController/BP_GPlayerController` (`self.GetController`)))
              (`PlayerController.K2_ClientPlayForceFeedback` _asbp_gplayer_controller "/Game/Framework/PlayerController/HE_Collision.HE_Collision" "None" false false false))
            (:`then_1`
              (if (`self.bIsGravityActive`) :!label _label_3
                (`AudioComponent.FadeIn` (`self.sg_GravityActive`) 0.1 1.0 0.0 "Linear"))))
          (else
            (`AudioComponent.SetBoolParameter` (`self.CollisionAudio`) "WeakCollision" true)
            (`AudioComponent.Play` (`self.CollisionAudio`) 0.0)
            (goto _label_3)))
        (else
          (set `/Game/Player/BaseGravitor/BP_Gravitor.SoundPlayed` false _asbp_gravitor)
          (if _returnvalue_2
            (goto _label_2)))))
    (:`CastFailed`
      (goto _label))))

(event `TickVFX`
  (params (DeltaTime :type "Float (double-precision)")))

(event `TickSFX`
  (`AudioComponent.SetBoolParameter` (`self.sg_GravityActive`) "BallInRange" (`self.bIsAttractingBall`))
  (`AudioComponent.SetBoolParameter` (`self.sg_GravityActive`) "IsPossessingBall" (`self.bIsOwningABall`))
  (if (`self.bIsGravityActive`)
    (`/Engine/EditorBlueprintResources/StandardMacros.DoOnce` false :!label _label_4
      (:`Completed`
        (`AudioComponent.FadeIn` (`self.sg_GravityActive`) 0.1 1.0 0.0 "Linear")
        (goto _label_5 :!via `Reset`)))
    (else
      (`/Engine/EditorBlueprintResources/StandardMacros.DoOnce` false :!label _label_5
        (:`Completed`
          (`AudioComponent.FadeOut` (`self.sg_GravityActive`) 0.2 0.0 "Linear")
          (goto _label_4 :!via `Reset`))))))

(fn `UserConstructionScript`)