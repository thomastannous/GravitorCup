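; Game mode for Gravity Ball that sets up the score and countdown UI and the grass-affector emitters.
; BeginPlay creates both widgets and caches the grass scene capture; round reset shows the countdown and round start hides it.
; For each player, it spawns an emitter following their Gravitor and another attached to the first ball.
; Emitters join the capture's show-only list, then the first controller hides capture components.
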(event `self.ReceiveBeginPlay`
  (`|ExecutionSequence`
    (:`then_0`
      (bind _returnvalue (`|CreateWidget` "/Game/GUI/DuringPlay/W_Score.W_Score_C"))
      (`UserWidget.AddToViewport` _returnvalue 0))
    (:`then_1`
      (bind _returnvalue_2 (`|CreateWidget` "/Game/GUI/DuringPlay/W_Countdown.W_Countdown_C"))
      (bind _output_get (set `self.CountdownWidget` _returnvalue_2))
      (`Widget.SetVisibility` _output_get "Hidden")
      (`UserWidget.AddToViewport` _output_get 0))
    (:`then_2`
      (bind _returnvalue_3 (`GameplayStatics.GetActorOfClass` "/Game/LevelContent/GGrass/GGrassSceneCap.GGrassSceneCap_C"))
      (set `self.CaptureComp` (`SceneCapture2D.CaptureComponent2D` _returnvalue_3)))))

(event `self.K2_OnRoundStart`
  (`Widget.SetVisibility` (`self.CountdownWidget`) "Hidden"))

(event `self.K2_OnRoundReset`
  (`Widget.SetVisibility` (`self.CountdownWidget`) "Visible"))

(event `self.SpawnGrassAffectorEmitters`
  (bind _output (`|GetArrayItem` (`self.Balls`)))
  (bind _asbp_gravity_ball_game_mode (cast `/Game/Framework/GameModes/BP_GravityBallGameMode` (`GameplayStatics.GetGameMode`)))
  (for _index (range (`GGameModeBase.DesiredPlayerNum` _asbp_gravity_ball_game_mode))
    (bind _asbp_gplayer_controller (cast `/Game/Framework/PlayerController/BP_GPlayerController` (`GameplayStatics.GetPlayerController` _index)))
    (bind _asbp_gravitor (cast `/Game/Player/BaseGravitor/BP_Gravitor` (`Controller.K2_GetPawn` _asbp_gplayer_controller)))
    (bind _returnvalue (`|SpawnActorFromClass` "/Game/LevelContent/GGrass/GravitorGrassEmitter.GravitorGrassEmitter_C" (`self.GetTransform` _asbp_gravitor) "AlwaysSpawn" "OverrideRootScale" (`GameplayStatics.GetPlayerController` 0) _asbp_gravitor))
    (set `/Game/LevelContent/GGrass/GravitorGrassEmitter.GravitorToFollow` _asbp_gravitor _returnvalue)
    (`SceneCaptureComponent.ShowOnlyActorComponents` (`self.CaptureComp`) _returnvalue false)
    (bind _returnvalue_2 (`|SpawnActorFromClass` "/Game/LevelContent/GGrass/BallGrassEmitter.BallGrassEmitter_C" (`self.GetTransform`) "Undefined" "OverrideRootScale" (`GameplayStatics.GetPlayerController` 0) null))
    (`self.K2_AttachToActor` _returnvalue_2 _output "None" "KeepRelative" "KeepRelative" "KeepRelative" true)
    (set `/Game/LevelContent/GGrass/BallGrassEmitter.Ball` _output _returnvalue_2)
    (`SceneCaptureComponent.ShowOnlyActorComponents` (`self.CaptureComp`) _returnvalue_2 false))
  (bind _asgplayer_controller (cast `GPlayerController` (`GameplayStatics.GetPlayerController` 0)))
  (`GPlayerController.HideCaptureComponents` _asgplayer_controller))

(fn `UserConstructionScript`)