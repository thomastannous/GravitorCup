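; Main menu game mode that shows the menu interface and relays player join and leave events to it.
; On BeginPlay it creates the W_MainMenu widget and adds it to the viewport.
; Join and leave events switch on the selected game mode, 1v1 or 2v2, and pass the player controller to the matching widget handler.
; The left and right team-selection input events are empty.
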(event `self.ReceiveBeginPlay`
  (bind _returnvalue (`|CreateWidget` "/Game/GUI/MainMenu/W_MainMenu.W_MainMenu_C"))
  (bind _output_get (set `self.MainMenuWidget` _returnvalue))
  (`UserWidget.AddToViewport` _output_get 0))

(event `self.PlayerInputLeftInTeamSelection`)

(event `self.PlayerInputRightInTeamSelection`)

(event `self.OnPlayerJoin`
  (params (GPlayerController :type "GPlayerController Object Reference"))
  (bind _mainmenuwidget (`self.MainMenuWidget`))
  (switch `ESelectedGameMode` (`self.SelectedGameMode`)
    (:`SG_1v1`
      (`/Game/GUI/MainMenu/W_MainMenu.1v1OnPlayerJoin` _mainmenuwidget GPlayerController))
    (:`SG_2v2`
      (`/Game/GUI/MainMenu/W_MainMenu.2v2OnPlayerJoin` _mainmenuwidget GPlayerController))))

(event `self.OnPlayerLeave`
  (params (GPlayerController :type "GPlayerController Object Reference"))
  (bind _mainmenuwidget (`self.MainMenuWidget`))
  (switch `ESelectedGameMode` (`self.SelectedGameMode`)
    (:`SG_1v1`
      (`/Game/GUI/MainMenu/W_MainMenu.1v1OnPlayerLeave` _mainmenuwidget GPlayerController))
    (:`SG_2v2`
      (`/Game/GUI/MainMenu/W_MainMenu.2v2OnPlayerLeave` _mainmenuwidget GPlayerController))))

(fn `UserConstructionScript`)